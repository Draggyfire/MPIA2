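; Enemy AI controller that walks its pawn along custom PathNode routes to the BP_Goal stone with the fewest path nodes, then to the hospital when carrying one.
; Tick steers straight at each node with movement input.
; If BP_ThirdPersonCharacter actors target the next node, it reroutes around it.
; Once stopped, after an initial one-second delay that never resets, it re-picks a route every tick.
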(event `self.ReceiveBeginPlay`
  (bind _outactors (`GameplayStatics.GetAllActorsOfClass` "/Game/Path/BP_Hopital.BP_Hopital_C"))
  (bind _returnvalue (`self.GetClosestPathNode` (`|GetArrayItem` _outactors)))
  (set `self.Hopital` _returnvalue)
  (bind (_stonenearestnode1 _path1) (`self.GetNearestStone` (`self.K2_GetPawn`)))
  (set `self.Checkpoints` _path1)
  (`self.SetNextGoal`))

(event `self.ReceiveTick`
  (params (DeltaSeconds :type "Float (single-precision)"))
  (bind _returnvalue (`self.K2_GetPawn`))
  (if (`self.Stop`)
    ; Check tout les 3 secondes
    (bind _output_get (set `self.TimeCheckStone` (+ DeltaSeconds (`self.TimeCheckStone`))))
    (if (>= _output_get 1.0)
      ; Si l'IA a déjà un patient on lui refait aller à l'hopital
      (bind _hasstonecharacter (`self.HasPawnStone`))
      (if _hasstonecharacter
        (`self.GoToHopital`)
        (else
          (bind (_stonenearestnode1 _path1) (`self.GetNearestStone` (`self.K2_GetPawn`)))
          (if (not (`KismetArrayLibrary.Array_IsEmpty` _path1))
            (set `self.Checkpoints` _path1)
            (set `self.Stop` false)
            (set `self.countCheckpoint` 0)))))
    (elif (!= (`self.Goal`) (`self.K2_GetActorLocation` (`self.K2_GetPawn`)) :`ErrorTolerance` 3.0)
      (`Pawn.AddMovementInput` _returnvalue (`KismetMathLibrary.Normal` (- (`self.Goal`) (`self.K2_GetActorLocation` _returnvalue))) 1.0 false)
      (else
        (`self.SetNextGoal`)))))

(event `SetNextGoal`
  (bind _checkpoints (`self.Checkpoints`))
  (bind _output (`|GetArrayItem` (`self.Checkpoints`) (`self.countCheckpoint`)))
  (if (> (`KismetArrayLibrary.Array_Length` (`self.Checkpoints`)) (`self.countCheckpoint`))
    (bind _aspath_node (cast `PathNode` _output))
    (bind _outactors (`GameplayStatics.GetAllActorsOfClass` "/Game/ThirdPerson/Blueprints/BP_ThirdPersonCharacter.BP_ThirdPersonCharacter_C"))
    (bind _returnvalue (`self.IsPathNodeTargeted` _aspath_node _outactors 100.0 180.0))
    (if _returnvalue
      (`BlueprintSetLibrary.Set_Clear` (`self.Blocked Nodes`))
      (`BlueprintSetLibrary.Set_Add` (`self.Blocked Nodes`) _aspath_node)
      (bind _aspath_node_2 (cast `PathNode` (`|GetArrayItem` _checkpoints (`KismetArrayLibrary.Array_LastIndex` _checkpoints))))
      (bind _returnvalue_2 (`self.GetClosestPathNode` (`self.K2_GetPawn`)))
      (bind _returnvalue_3 (`self.FindPathWithBlockedNodes` _returnvalue_2 _aspath_node_2 (`self.Blocked Nodes`)))
      (bind _output_get (set `self.Checkpoints` _returnvalue_3))
      (`BlueprintSetLibrary.Set_Clear` (`self.Blocked Nodes`))
      (if (> (`KismetArrayLibrary.Array_Length` _output_get) 0)
        (set `self.Goal` (`self.K2_GetActorLocation` (`|GetArrayItem` _output_get)))
        (set `self.countCheckpoint` 0)
        (else
          (set `self.Stop` true)))
      (else
        (set `self.Goal` (`self.K2_GetActorLocation` _output))
        (set `self.countCheckpoint` (+ (`self.countCheckpoint`) 1))))
    (else
      (set `self.Stop` true))))

(event `GoToHopital`
  (set `self.Stop` false)
  (set `self.countCheckpoint` 0)
  (bind _returnvalue (`self.GetClosestPathNode` (`self.K2_GetPawn`)))
  (bind _returnvalue_2 (`self.FindPath` _returnvalue (`self.Hopital`)))
  (set `self.Checkpoints` _returnvalue_2))

(fn `GetNearestStone`
  (params (FromActor :type "Actor Object Reference"))
  (returns (StoneNearestNode1 :type "/Game/Path/BP_Goal Object Reference") (Path1 :type "Array of PathNode Object Reference"))
  (locals (NbPathnode :type Integer :default 999) (StoneNearestNode :type "/Game/Path/BP_Goal Object Reference") (Path :type "Array of PathNode Object Reference") (Actor :type "Actor Object Reference"))
  (set `local.Actor` FromActor)
  (bind _outactors (`GameplayStatics.GetAllActorsOfClass` "/Game/Path/BP_Goal.BP_Goal_C"))
  (for _array_element _outactors
    (bind _path (`self.GetPath` (`local.Actor`) _array_element))
    (bind _returnvalue (`KismetArrayLibrary.Array_Length` _path))
    (if (and (< _returnvalue (`local.NbPathnode`)) (not (`KismetArrayLibrary.Array_IsEmpty` _path)))
      (set `local.NbPathnode` _returnvalue)
      (set `local.StoneNearestNode` _array_element)
      (set `local.Path` _path)))
  (return (`local.StoneNearestNode`) (`local.Path`)))

(fn `GetPath`
  (params (FromActor :type "Actor Object Reference") (FromActor1 :type "Actor Object Reference"))
  (returns (Path :type "Array of PathNode Object Reference"))
  (bind _returnvalue (`self.GetClosestPathNode` FromActor))
  (bind _returnvalue_2 (`self.GetClosestPathNode` FromActor1))
  (bind _returnvalue_3 (`self.FindPath` _returnvalue _returnvalue_2))
  (return _returnvalue_3))

(fn `HasPawnStone`
  (returns (hasStoneCharacter :type Boolean))
  (bind _asbp_enemy (cast `/Game/ThirdPerson/Blueprints/BP_Enemy` (`self.K2_GetPawn`)))
  (return (`/Game/ThirdPerson/Blueprints/BP_Enemy.hasStoneCharacter` _asbp_enemy)))

(fn `UserConstructionScript`)