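; BP_Goal is a pickup that hands the stone character to whoever first touches its sphere collider, enemy or player.
; On overlap, an enemy or third-person character not already carrying one has its stone character visibility switched, and the goal destroys itself.
; For an enemy, it then tells that enemy's BP_EnemyController to go to the hospital.
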(event `self.SphereCollider.OnComponentBeginOverlap`
  (params (OverlappedComponent :type "PrimitiveComponent Object Reference") (OtherActor :type "Actor Object Reference") (OtherComp :type "PrimitiveComponent Object Reference") (OtherBodyIndex :type Integer) (bFromSweep :type Boolean) (SweepResult :type "HitResult Structure (by ref)"))
  (bind _asbp_enemy (cast `/Game/ThirdPerson/Blueprints/BP_Enemy` OtherActor)
    (:`then`
      (if (not (`/Game/ThirdPerson/Blueprints/BP_Enemy.hasStoneCharacter` _asbp_enemy))
        (`/Game/ThirdPerson/Blueprints/BP_Enemy.SwitchStoneCharacterVisibility` _asbp_enemy)
        (`self.K2_DestroyActor`)
        (bind _asbp_enemy_controller (cast `/Game/Controller/BP_EnemyController` (`Pawn.GetController` _asbp_enemy)))
        (`/Game/Controller/BP_EnemyController.GoToHopital` _asbp_enemy_controller)))
    (:`CastFailed`
      (bind _asbp_third_person_character (cast `/Game/ThirdPerson/Blueprints/BP_ThirdPersonCharacter` OtherActor))
      (if (not (`/Game/ThirdPerson/Blueprints/BP_ThirdPersonCharacter.hasStoneCharacter` _asbp_third_person_character))
        (`/Game/ThirdPerson/Blueprints/BP_ThirdPersonCharacter.SwitchStoneCharacterVisibility` _asbp_third_person_character)
        (`self.K2_DestroyActor`)))))

(fn `UserConstructionScript`)